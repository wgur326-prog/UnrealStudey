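; BP_Button is an overlap-activated button that oscillates a Target actor while something is inside its Box.
; While overlapped, Tick accumulates Time and adds a sine offset, scaled by MoveLength and MoveSpeed, to the Target's current location along world X or Y, chosen by ButtonType.
; Ending the overlap snaps the Target to StartLocation, which this graph never assigns, and leaves Time unreset.
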(event OnComponentBeginOverlap(Box)
  (params (OverlappedComponent :type Primitive%20Component%20Object%20Reference) (OtherActor :type Actor%20Object%20Reference) (OtherComp :type Primitive%20Component%20Object%20Reference) (OtherBodyIndex :type Integer) (bFromSweep :type Boolean) (SweepResult :type Hit%20Result%20Structure%20%28by%20ref%29))
  (Variables|Default|SetbIsOverlap true))

(event OnComponentEndOverlap(Box)
  (params (OverlappedComponent :type Primitive%20Component%20Object%20Reference) (OtherActor :type Actor%20Object%20Reference) (OtherComp :type Primitive%20Component%20Object%20Reference) (OtherBodyIndex :type Integer))
  (Variables|Default|SetbIsOverlap false)
  (Transformation|SetActorLocation (Variables|Default|GetTarget) (Variables|Default|GetStartLocation) false false))

(event EventTick
  (params (DeltaSeconds :type Float%20%28single-precision%29))
  (if (Variables|Default|GetbIsOverlap)
    (bind _output_get (Variables|Default|SetTime (+ DeltaSeconds (Variables|Default|GetTime))))
    (if (Utilities|Enum|Equal(Enum) (Variables|Default|GetButtonType) "NewEnumerator0")
      (Transformation|SetActorLocation (Variables|Default|GetTarget) (+ (Transformation|GetActorLocation (Variables|Default|GetTarget)) (Math|Vector|MakeVector (* (Variables|Default|GetMoveLength) (Math|Trig|Sin(Radians) (* _output_get (Variables|Default|GetMoveSpeed)))) 0.0 0.0)) false false)
      (else
        (Transformation|SetActorLocation (Variables|Default|GetTarget) (+ (Transformation|GetActorLocation (Variables|Default|GetTarget)) (Math|Vector|MakeVector 0.0 (* (Variables|Default|GetMoveLength) (Math|Trig|Sin(Radians) (* _output_get (Variables|Default|GetMoveSpeed)))) 0.0)) false false)))))

(fn ConstructionScript)