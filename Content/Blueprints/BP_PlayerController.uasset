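; BP_PlayerController is a player controller that translates input into movement, look, jump and fire for the player character.
; Turn and Lookup axes add yaw and pitch input, while move axes add movement input to pawn 0 along the controller's own forward and right vectors.
; Jump calls the character's built-in Jump, and Fire casts the character to BP_Player and calls its Fire function.
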(event Input|ActionEvents|InputActionJump
  (params (Key :type Key%20Structure :default "None"))
  ;[0.15 0.15 0.15 0.5] 점프
  (:Pressed
    (Character|Jump (Game|GetPlayerCharacter 0))))

(event Input|ActionEvents|InputActionFire
  (params (Key :type Key%20Structure :default "None"))
  ;[0.15 0.15 0.15 0.5] 공격
  ;;[0.15 0.15 0.15 0.5] 왼쪽 마우스 누르면 실행
  (:Pressed
    ;;[0.15 0.15 0.15 0.5] 캐릭터라는 자료형을 BP_Player로 변환
    (bind _asbp_player (Utilities|Casting|CastToBP_Player (Game|GetPlayerCharacter 0)))
    ;;[0.15 0.15 0.15 0.5] 변환에 성공했으면 걔가 갖고있는 Fire 라는 함수를 실행한다
    (Default|Fire _asbp_player)))

(event Input|AxisEvents|InputAxisMoveForward
  (params (AxisValue :type Float%20%28single-precision%29))
  ;[0.15 0.15 0.15 0.5] 플레이어 이동
  ;;[0.15 0.15 0.15 0.5] 이동시키는 함수가 아님
  (Pawn|Input|AddMovementInput (Game|Player|GetPlayerPawn 0) (Transformation|GetActorForwardVector) AxisValue false))

(event Input|AxisEvents|InputAxisMoveRight
  (params (AxisValue :type Float%20%28single-precision%29))
  ;[0.15 0.15 0.15 0.5] 플레이어 이동
  (Pawn|Input|AddMovementInput (Game|Player|GetPlayerPawn 0) (Transformation|GetActorRightVector) AxisValue false))

(event Input|AxisEvents|InputAxisTurn
  (params (AxisValue :type Float%20%28single-precision%29))
  ;[0.15 0.15 0.15 0.5] 플레이어 회전
  (Class|PlayerController|AddYawInput AxisValue))

(event Input|AxisEvents|InputAxisLookup
  (params (AxisValue :type Float%20%28single-precision%29))
  ;[0.15 0.15 0.15 0.5] 플레이어 회전
  (Class|PlayerController|AddPitchInput AxisValue))

(fn ConstructionScript)