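; BP_Red is a trigger box that slides a referenced Target actor while something overlaps it.
; Box overlap events toggle IsOverlapping, and Tick moves Target a fixed step along negative Y while it is true, without delta-time scaling or sweep.
; End overlap clears the flag and snaps Target back to StartLocation.
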(event OnComponentBeginOverlap(Box)
  (params (OverlappedComponent :type Primitive%20Component%20Object%20Reference) (OtherActor :type Actor%20Object%20Reference) (OtherComp :type Primitive%20Component%20Object%20Reference) (OtherBodyIndex :type Integer) (bFromSweep :type Boolean) (SweepResult :type Hit%20Result%20Structure%20%28by%20ref%29))
  (Variables|Default|SetIsOverlapping true))

(event OnComponentEndOverlap(Box)
  (params (OverlappedComponent :type Primitive%20Component%20Object%20Reference) (OtherActor :type Actor%20Object%20Reference) (OtherComp :type Primitive%20Component%20Object%20Reference) (OtherBodyIndex :type Integer))
  (Variables|Default|SetIsOverlapping false)
  (Transformation|SetActorLocation (Variables|Default|GetTarget) (Variables|Default|GetStart%20Location) false false))

(event EventTick
  (params (DeltaSeconds :type Float%20%28single-precision%29))
  (if (Variables|Default|GetIsOverlapping)
    (Transformation|SetActorLocation (Variables|Default|GetTarget) (+ (Transformation|GetActorLocation (Variables|Default|GetTarget)) "0.000000,-1.000000,0.000000") false false)))

(fn ConstructionScript)