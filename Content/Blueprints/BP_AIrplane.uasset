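; Airplane actor that moves along its forward vector every Tick and rotates its static mesh from axis input.
; Movement is an unswept one-unit step per frame; the Speed and DeltaSeconds scaling is left unconnected.
; LeftRotation and RightRotation axes both feed AddRotation, which applies local pitch scaled by RotateSpeed and the stored DeltaSeconds.
; BeginPlay also swaps A and B by reference and prints them.
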(event EventTick
  (params (DeltaSeconds :type Float%20%28single-precision%29))
  ;[0.15 0.15 0.15 0.5] 액터가 바라보는 정면 방향으로 이동하겠다
  (bind _output_get (Variables|Default|SetDelta%20Seconds DeltaSeconds))
  ;;[0.15 0.15 0.15 0.5] 월드좌표를 기준으로 새 좌표로 이동하겠다
  (Transformation|SetActorLocation (+ (Transformation|GetActorLocation) (Transformation|GetActorForwardVector)) false false))

(event EventBeginPlay
  (CallFunction|Swap (Variables|Default|GetA) (Variables|Default|GetB))
  (Development|PrintText (Utilities|Text|FormatText "A: {A}, B : {B}" (Variables|Default|GetA) (Variables|Default|GetB)) true true "(R=0.000000,G=0.660000,B=1.000000,A=1.000000)" 9999.0))

(event Input|AxisEvents|InputAxisLeftRotation
  (params (AxisValue :type Float%20%28single-precision%29))
  ;[0.15 0.15 0.15 0.5] 액터가 바라보는 정면 방향으로 이동하겠다
  ;;[0.15 0.15 0.15 0.5] 멤버함수
  (CallFunction|AddRotation AxisValue))

(event Input|AxisEvents|InputAxisRightRotation
  (params (AxisValue :type Float%20%28single-precision%29))
  ;[0.15 0.15 0.15 0.5] 액터가 바라보는 정면 방향으로 이동하겠다
  ;;[0.15 0.15 0.15 0.5] 멤버함수
  (CallFunction|AddRotation AxisValue))

(fn ConstructionScript)

(fn AddRotation
  (params (AxisVal :type Float%20%28double-precision%29))
  (Transformation|AddLocalRotation (Variables|Default|GetStaticMesh) (Math|Rotator|MakeRotator 0.0 (* AxisVal (Variables|Default|GetDelta%20Seconds) (Variables|Default|GetRotateSpeed)) 0.0) false false))

(fn Swap
  (params (FuncA :type Integer%20%28by%20ref%29) (FuncB :type Integer%20%28by%20ref%29))
  (bind _output_get (LocalVariables|SetTemp2 FuncA))
  (|SetBy-RefVar FuncA FuncB)
  (|SetBy-RefVar FuncB _output_get))